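; Small coin collectible that defines a random currency value and pickup message for a parent pickup class.
; The construction script rolls an amount between 100 and 200, truncated to two decimal places, and builds a pound-prefixed message from it.
; It sets both variables before calling the parent construction script, and its own event graph holds only disabled stub events.
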(event EventBeginPlay
  (|CallParentFunction) ; This node is disabled and will not be called.\nDrag off pins to build functionality.
)

(event Collision|EventActorBeginOverlap
  (params (OtherActor :type Actor%20Object%20Reference))
  (|CallParentFunction OtherActor) ; This node is disabled and will not be called.\nDrag off pins to build functionality.
)

(event EventTick
  (params (DeltaSeconds :type Float%20%28single-precision%29))
  (|CallParentFunction DeltaSeconds) ; This node is disabled and will not be called.\nDrag off pins to build functionality.
)

(fn ConstructionScript
  (Variables|Default|SetCurrencyToAdd (/ (Math|Conversions|ToFloat(Integer) (Math|Float|Truncate (* (Math|Random|RandomFloatinRange 1e+02 2e+02) 1e+02))) 1e+02))
  (Variables|Default|SetPickupMessage (Utilities|String|Append "£" (Utilities|String|ToString(Float) (Variables|Default|GetCurrencyToAdd))))
  (|CallParentFunction))