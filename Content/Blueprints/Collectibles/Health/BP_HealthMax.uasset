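; BP_HealthMax is a health collectible that fully restores the health of the character that picks it up.
; It overrides the inherited OnPickup event to set the character's CurrentHealth to its MaxHealth, then calls the parent implementation for the remaining pickup handling.
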(event EventBeginPlay
  (|CallParentFunction) ; This node is disabled and will not be called.\nDrag off pins to build functionality.
)

(event Collision|EventActorBeginOverlap
  (params (OtherActor :type Actor%20Object%20Reference))
  (|CallParentFunction OtherActor) ; This node is disabled and will not be called.\nDrag off pins to build functionality.
)

(event EventTick
  (params (DeltaSeconds :type Float%20%28single-precision%29))
  (|CallParentFunction DeltaSeconds) ; This node is disabled and will not be called.\nDrag off pins to build functionality.
)

(event EventOnPickup
  (params (Character :type BP%20First%20Person%20Character%20Object%20Reference))
  ;[1 1 1] Overide On Pickup function to set Current health to Max Health
  (Variables|/Game/Blueprints/BP_FirstPersonCharacter.BP_FirstPersonCharacter_C|SetCurrentHealth Character (Variables|/Game/Blueprints/BP_FirstPersonCharacter.BP_FirstPersonCharacter_C|GetMaxHealth Character))
  (|CallParentFunction Character))

(fn ConstructionScript
  (|CallParentFunction))