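; BP_BaseHealth is a base health collectible that restores a character's health when picked up.
; OnPickup adds HealthToAdd, which the author's comment says comes from child classes, to CurrentHealth, clamps it between zero and MaxHealth, then calls the parent pickup event.
; The CanBePickedUp override calls the parent but ignores its result, refusing pickup only when CurrentHealth equals MaxHealth.
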(event EventOnPickup
  (params (Character :type BP%20First%20Person%20Character%20Object%20Reference))
  ;[1 1 1] Call "OnPickup" event to get Current Health, add Health to Add from child class, clamp to ensure it goes no higher than max health. Set Current Health
  (Variables|/Game/Blueprints/BP_FirstPersonCharacter.BP_FirstPersonCharacter_C|SetCurrentHealth Character (Math|Float|Clamp(Float) (+ (Variables|/Game/Blueprints/BP_FirstPersonCharacter.BP_FirstPersonCharacter_C|GetCurrentHealth Character) (Variables|Default|GetHealthToAdd)) 0.0 (Variables|/Game/Blueprints/BP_FirstPersonCharacter.BP_FirstPersonCharacter_C|GetMaxHealth Character)))
  (|CallParentFunction Character))

(fn ConstructionScript
  (|CallParentFunction))

(fn CanbePickedUp
  (params (Character :type BP%20First%20Person%20Character%20Object%20Reference))
  ;[1 1 1] Overide "CanBePickedUpFunction" to check if Current Health is = to Max Health. If it is, do not carry out function. If not, pick up health.
  (|CallParentFunction Character)
  (if (== (Variables|/Game/Blueprints/BP_FirstPersonCharacter.BP_FirstPersonCharacter_C|GetMaxHealth Character) (Variables|/Game/Blueprints/BP_FirstPersonCharacter.BP_FirstPersonCharacter_C|GetCurrentHealth Character))
    (return false)
    (else
      (return true))))