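; Base Blueprint for shield collectibles that add ShieldsToAdd, an amount set by child classes, to the character's CurrentShield.
; OnPickup clamps the new total between zero and MaxShield, then calls the parent pickup logic.
; The CanBePickedUp override refuses pickup whenever the full amount would exceed MaxShield, ignoring the parent's result, so partial top-ups are not allowed.
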(event EventOnPickup
  (params (Character :type BP%20First%20Person%20Character%20Object%20Reference))
  ;[1 1 1] Call "OnPickup" event to get current shield, add shield to add from child class, clamp to ensure it goes no higher than max shield
  (Variables|/Game/Blueprints/BP_FirstPersonCharacter.BP_FirstPersonCharacter_C|SetCurrentShield Character (Math|Integer|Clamp(Integer) (+ (Variables|/Game/Blueprints/BP_FirstPersonCharacter.BP_FirstPersonCharacter_C|GetCurrentShield Character) (Variables|Default|GetShieldsToAdd)) 0 (Variables|/Game/Blueprints/BP_FirstPersonCharacter.BP_FirstPersonCharacter_C|GetMaxShield Character)))
  (|CallParentFunction Character))

(fn ConstructionScript
  (|CallParentFunction))

(fn CanbePickedUp
  (params (Character :type BP%20First%20Person%20Character%20Object%20Reference))
  ;[1 1 1] Overide "CanBePickedUpFunction" to check if adding shield will be more than Max Shield. If it is, do not carry out function
  (|CallParentFunction Character)
  (if (> (+ (Variables|/Game/Blueprints/BP_FirstPersonCharacter.BP_FirstPersonCharacter_C|GetCurrentShield Character) (Variables|Default|GetShieldsToAdd)) (Variables|/Game/Blueprints/BP_FirstPersonCharacter.BP_FirstPersonCharacter_C|GetMaxShield Character))
    (return false)
    (else
      (return true))))